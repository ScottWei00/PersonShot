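; Base weapon Blueprint for the PersonShot game, handling firing, ammo and reloading.
; WeaponFire runs AmmoCheck for sound and ammo count, then a camera-forward line trace with random spread, even when empty.
; The trace only draws debug lines, as its hit is unused and SpawnDecalTracer is an empty stub.
; WeaponReload refills the magazine before computing the reserve deduction, so MaxAmmo never drops.
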(event `WeaponFire`
  (`self.AmmoCheck`)
  (`self.LineTrace`)
  (`self.SpawnDecalTracer`))

(event `WeaponReload`
  (if (and (> (`self.MaxAmmo`) 0) (< (`self.CurrentAmmo`) (`self.AmmoCount`)))
    (set `self.CurrentAmmo` (`self.AmmoCount`))
    (set `self.MaxAmmo` (- (`self.MaxAmmo`) (- (`self.AmmoCount`) (`self.CurrentAmmo`))))
    (`GameplayStatics.PlaySoundAtLocation` "/Game/PersonShot/audios/Reload_Load.Reload_Load" (0.0 0.0 0.0) (struct) 1.0 1.0 0.0 null null null)))

(fn `AmmoCheck`
  (bind _currentammo (`self.CurrentAmmo`))
  (if (> (`self.CurrentAmmo`) 0)
    (`GameplayStatics.PlaySoundAtLocation` "/Game/FirstPerson/Audio/FirstPersonTemplateWeaponFire02.FirstPersonTemplateWeaponFire02" (0.0 0.0 0.0) (struct) 1.0 1.0 0.0 null null null)
    (`/Engine/EditorBlueprintResources/StandardMacros.DecrementInt` _currentammo
      (:`  `
        (`KismetSystemLibrary.PrintString` (`KismetStringLibrary.Conv_IntToString` _currentammo))))
    (else
      (`GameplayStatics.PlaySoundAtLocation` "/Game/PersonShot/audios/DryFire.DryFire" (0.0 0.0 0.0) (struct) 1.0 1.0 0.0 null null null))))

(fn `LineTrace`
  (bind _bulletspread (`self.BulletSpread`))
  (bind _followcamera (`/Game/PersonShot/Blueprints/PersonShot.FollowCamera` (cast `/Game/PersonShot/Blueprints/PersonShot` (`GameplayStatics.GetPlayerCharacter` 0) :!pure true)))
  (bind _returnvalue (`SceneComponent.K2_GetComponentLocation` _followcamera))
  (bind _outhit (`KismetSystemLibrary.LineTraceSingle` :`Start` _returnvalue :`End` (+ _returnvalue (+ (* (`SceneComponent.GetForwardVector` _followcamera) 20000.0) (`KismetMathLibrary.MakeVector` (`KismetMathLibrary.RandomFloatInRange` (* _bulletspread -1.0) _bulletspread) (`KismetMathLibrary.RandomFloatInRange` (* _bulletspread -1.0) _bulletspread) (`KismetMathLibrary.RandomFloatInRange` (* _bulletspread -1.0) _bulletspread)))) :`TraceChannel` "TraceTypeQuery1" :`DrawDebugType` "ForDuration" :`DrawTime` 2.0)))

(fn `SpawnDecalTracer`)

(fn `UserConstructionScript`
  (set `self.MaxAmmo` 200)
  (set `self.AmmoCount` 30)
  (set `self.CurrentAmmo` 30)
  (set `self.BulletSpread` 500.0)
  (set `self.ReloadTime` 2.0))